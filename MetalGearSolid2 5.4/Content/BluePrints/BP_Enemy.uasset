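; Enemy Blueprint with a rifle, a health bar widget and Gameplay Ability System support, granting its listed abilities on BeginPlay.
; The health bar turns toward the player camera each tick, and Fire plays a montage with muzzle flash and sound.
; Damage alerts the AI controller to the instigator pawn's location, then lowers health.
; Survivable hits trigger a Damaged ability; death adds a Dead tag, hides the bar, ragdolls and sets a lifespan.
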(event `self.ReceiveBeginPlay`
  (bind _asui_enemy_hpbar (cast `/Game/UI/UI_EnemyHPbar` (`WidgetComponent.GetUserWidgetObject` (`self.EnemyHPbar`))))
  (set `/Game/UI/UI_EnemyHPbar.BP_Enemy` self _asui_enemy_hpbar)
  (for _array_element (`self.Ability`)
    (`AbilitySystemComponent.K2_GiveAbility` (`self.AbilitySystem`) _array_element 0 -1)))

(event `self.ReceiveTick`
  (params (DeltaSeconds :type "Float (single-precision)"))
  (`self.WidgetRotation`))

(event `WidgetRotation`
  (`SceneComponent.K2_SetWorldRotation` (`self.EnemyHPbar`) (`KismetMathLibrary.FindLookAtRotation` (`SceneComponent.K2_GetComponentLocation` (`self.EnemyHPbar`)) (`self.K2_GetActorLocation` (`GameplayStatics.GetPlayerCameraManager` 0))) false false))

(event `Fire`
  (bind (_returnvalue_location _returnvalue_rotation) (`KismetMathLibrary.BreakTransform` (`SceneComponent.GetSocketTransform` (`self.Rifle`) "MuzzleFlash" "RTS_World")))
  (`|PlayMontage` (`self.Mesh`) "/Game/Characters/Enemy/AnimMontage/MM_Rifle_Fire_Montage.MM_Rifle_Fire_Montage"
    (:`then`
      (`GameplayStatics.SpawnEmitterAtLocation` "/Game/MilitaryWeapSilver/FX/P_AssaultRifle_MuzzleFlash.P_AssaultRifle_MuzzleFlash" _returnvalue_location _returnvalue_rotation)
      (`GameplayStatics.PlaySoundAtLocation` "/Game/MilitaryWeapSilver/Sound/Rifle/Cues/RifleA_Fire_Cue.RifleA_Fire_Cue" _returnvalue_location (struct) 1.0 1.0 0.0 null null null null))))

(event `TakeDamage`
  (params (Damage :type "Float (double-precision)") (Instigator :type "Controller Object Reference"))
  (bind _output_get (set `self.Health` (`KismetMathLibrary.FClamp` (- (`self.Health`) Damage) 0.0 100.0)))
  (set `self.HealthPercentage` (/ _output_get 100.0))
  (if (<= (`self.Health`) 0.0)
    (`AbilitySystemBlueprintLibrary.AddLooseGameplayTags` self (`BlueprintGameplayTagLibrary.MakeLiteralGameplayTagContainer` (struct :`GameplayTags` (struct :`(TagName` "Ability.State.Dead")))))
    (`SceneComponent.SetVisibility` (`self.EnemyHPbar`) false false)
    (`SkeletalMeshComponent.SetAllBodiesSimulatePhysics` (`self.Mesh`) true)
    (`PrimitiveComponent.SetCollisionEnabled` (`self.Mesh`) "QueryAndPhysics")
    (`self.SetLifeSpan` (`self.LifeSpan`))
    (else
      (`AbilitySystemComponent.TryActivateAbilitiesByTag` (`self.AbilitySystem`) (`BlueprintGameplayTagLibrary.MakeLiteralGameplayTagContainer` (struct :`GameplayTags` (struct :`(TagName` "Ability.Action.Damaged")))) true))))

(event `self.ReceiveAnyDamage`
  (params (Damage :type "Float (single-precision)") (DamageType :type "DamageType Object Reference") (InstigatedBy :type "Controller Object Reference") (DamageCauser :type "Actor Object Reference"))
  (bind _asbp_aicontroller (cast `/Game/BluePrints/AI/BP_AIController` (`AIBlueprintHelperLibrary.GetAIController` self)))
  (`/Game/BluePrints/AI/BP_AIController.OnDamagePerception` _asbp_aicontroller (`self.K2_GetActorLocation` (`Controller.K2_GetPawn` InstigatedBy)))
  (`KismetSystemLibrary.PrintString` "Hit!")
  (`self.TakeDamage` Damage InstigatedBy))

(fn `UserConstructionScript`)